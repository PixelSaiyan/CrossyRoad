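; Road terrain strip for a Crossy Road style game that spawns traffic and scores the player's crossing.
; On BeginPlay it picks one traffic direction, then a looping timer with a randomized interval randomly spawns cars at the matching end marker.
; The player's first hit on the Cube updates their score and starts a recurring check that destroys the strip once the player is far enough ahead along X.
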(event OnComponentHit(Cube)
  (params (HitComponent :type Primitive%20Component%20Object%20Reference) (OtherActor :type Actor%20Object%20Reference) (OtherComp :type Primitive%20Component%20Object%20Reference) (NormalImpulse :type Vector :default "0, 0, 0") (Hit :type Hit%20Result%20Structure%20%28by%20ref%29))
  (bind _asthird_person_character (Utilities|Casting|CastToThirdPersonCharacter OtherActor))
  (Utilities|FlowControl|DoOnce false
    (:Completed
      (Default|UpdateScore _asthird_person_character)
      (Utilities|Time|SetTimerbyEvent (delegate Custom|Destroy) 5.0 true))))

(event Custom|Destroy
  (if (> (- (.x (Transformation|GetActorLocation (stale OnComponentHit(Cube) _asthird_person_character))) (.x (Transformation|GetActorLocation))) 2e+03)
    (Actor|DestroyActor)))

(event Custom|SpawnVehicle
  (if (Math|Random|RandomBool)
    (if (Variables|Default|GetVechileSpawn%20Direction)
      _
      (else
        _))
    (if (Variables|Default|GetVechileSpawn%20Direction)
      (Game|SpawnActorfromClass "/Game/CrossyRoadGame/Blueprints/Car.Car_C" (Math|Transform|MakeTransform (Variables|Default|GetStart%20Location) "0.000000,90.000000,0.000000" "1,1,1") "Undefined" 0 0)
      (else
        (Game|SpawnActorfromClass "/Game/CrossyRoadGame/Blueprints/Car.Car_C" (Math|Transform|MakeTransform (Variables|Default|GetEnd%20Location) "0.000000,-90.000000,0.000000" "1,1,1") "Undefined" 0 0)))))

(event EventBeginPlay
  (bind _start (Variables|Default|GetStart))
  (bind _start1 (Variables|Default|GetStart1))
  (bind _returnvalue (Transformation|GetWorldLocation _start))
  (bind _returnvalue_2 (Transformation|GetWorldLocation _start1))
  (Variables|Default|SetStart%20Location (Math|Vector|MakeVector (.x _returnvalue) (.y _returnvalue) (.z _returnvalue)))
  (Variables|Default|SetEnd%20Location (Math|Vector|MakeVector (.x _returnvalue_2) (.y _returnvalue_2) (.z _returnvalue_2)))
  (Variables|Default|SetVechileSpawn%20Direction (Math|Random|RandomBool))
  (Utilities|Time|SetTimerbyEvent (delegate Custom|SpawnVehicle) (Math|Random|RandomFloatinRange 2.0 3.5) true))

(event Collision|EventActorBeginOverlap
  (params (OtherActor :type Actor%20Object%20Reference)))

(fn ConstructionScript)