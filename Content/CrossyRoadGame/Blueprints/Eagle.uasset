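; Eagle hazard actor for the Crossy Road game that flies on projectile movement and kills the player it touches.
; On BeginPlay it sets extremely large random initial and max speeds, then destroys itself after a fixed delay, with a spotlight hide call placed after the destroy.
; Its box overlap casts the other actor to PlayerCharacter and calls DeathByEagle on it.
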(event OnComponentBeginOverlap(Box)
  (params (OverlappedComponent :type Primitive%20Component%20Object%20Reference) (OtherActor :type Actor%20Object%20Reference) (OtherComp :type Primitive%20Component%20Object%20Reference) (OtherBodyIndex :type Integer) (bFromSweep :type Boolean) (SweepResult :type Hit%20Result%20Structure%20%28by%20ref%29))
  (bind _asplayer_character (Utilities|Casting|CastToPlayerCharacter OtherActor))
  (Default|DeathbyEagle _asplayer_character))

(event EventBeginPlay
  (bind _returnvalue (Math|Random|RandomFloatinRange 9.799999488e+10 99999997952.0))
  (bind _projectilemovement (Variables|Default|GetProjectileMovement))
  (Variables|/Script/Engine.ProjectileMovementComponent|SetInitialSpeed _projectilemovement _returnvalue)
  (Variables|/Script/Engine.ProjectileMovementComponent|SetMaxSpeed _projectilemovement _returnvalue)
  (Utilities|FlowControl|Delay 14.0)
  (Actor|DestroyActor)
  (Rendering|SetVisibility (Variables|Default|GetSpot%20Light) false false))

(fn ConstructionScript)