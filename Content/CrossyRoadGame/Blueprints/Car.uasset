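; Crossy Road-style traffic vehicle that moves by ProjectileMovement and hits the player on contact.
; On BeginPlay a random roll picks one of four car meshes or a slower red truck, randomizes speed, then destroys the actor after a fixed delay.
; The roll's third outcome has no branch, leaving default mesh and speed with no timed destruction.
; Box overlap with the ThirdPersonCharacter calls its HitByVechile.
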(event OnComponentBeginOverlap(Box)
  (params (OverlappedComponent :type Primitive%20Component%20Object%20Reference) (OtherActor :type Actor%20Object%20Reference) (OtherComp :type Primitive%20Component%20Object%20Reference) (OtherBodyIndex :type Integer) (bFromSweep :type Boolean) (SweepResult :type Hit%20Result%20Structure%20%28by%20ref%29))
  (bind _asthird_person_character (Utilities|Casting|CastToThirdPersonCharacter OtherActor))
  (Default|HitbyVechile _asthird_person_character))

(event EventBeginPlay
  (bind _returnvalue (Math|Random|RandomFloatinRange 3e+02 3.3e+02))
  (bind _returnvalue_2 (Math|Random|RandomFloatinRange 2.5e+02 2.8e+02))
  (bind _projectilemovement (Variables|Default|GetProjectileMovement))
  (bind _projectilemovement_2 (Variables|Default|GetProjectileMovement))
  (switch int (Math|Random|RandomIntegerinRange 0 2)
    (:0
      (Components|StaticMesh|SetStaticMesh (Variables|Default|Getcar) (Utilities|Select :Index (Math|Random|RandomIntegerinRange 0 3) :Option%200 "/Game/Models/GreenCar/CrossyRoadGreenCar.CrossyRoadGreenCar" :Option%201 "/Game/Models/PoliceCar/CrossyRoadPoliceCar.CrossyRoadPoliceCar" :Option%202 "/Game/Models/BlueCar/CrossyRoadBlueCar.CrossyRoadBlueCar" :Option%203 "/Game/Models/PurpleCar/CrossyRoadPurpleCar.CrossyRoadPurpleCar"))
      (Variables|/Script/Engine.ProjectileMovementComponent|SetInitialSpeed _projectilemovement_2 _returnvalue)
      (Variables|/Script/Engine.ProjectileMovementComponent|SetMaxSpeed _projectilemovement_2 _returnvalue)
      (Utilities|FlowControl|Delay 14.0)
      (Actor|DestroyActor))
    (:1
      (Components|StaticMesh|SetStaticMesh (Variables|Default|Getcar) "/Game/Models/RedTruck/CrossyRoadRedTruck.CrossyRoadRedTruck")
      (Variables|/Script/Engine.ProjectileMovementComponent|SetInitialSpeed _projectilemovement _returnvalue_2)
      (Variables|/Script/Engine.ProjectileMovementComponent|SetMaxSpeed _projectilemovement _returnvalue_2)
      (Utilities|FlowControl|Delay 14.0)
      (Actor|DestroyActor))))

(fn ConstructionScript)