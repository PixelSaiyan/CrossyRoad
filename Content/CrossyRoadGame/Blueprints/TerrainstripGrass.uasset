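; Grass terrain strip for a Crossy Road-style game that populates itself, scores the player and cleans up behind them.
; BeginPlay steps between two markers along Y, randomly spawning an actor (no class shown) or a rare half-scale Coin.
; The player's first hit on the Cube updates the score and starts a looping timer that destroys the strip once left far behind.
; Overlapping either Deathbox triggers the player's off-screen death.
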(event OnComponentHit(Cube)
  (params (HitComponent :type Primitive%20Component%20Object%20Reference) (OtherActor :type Actor%20Object%20Reference) (OtherComp :type Primitive%20Component%20Object%20Reference) (NormalImpulse :type Vector :default "0, 0, 0") (Hit :type Hit%20Result%20Structure%20%28by%20ref%29))
  (bind _asplayer_character (Utilities|Casting|CastToPlayerCharacter OtherActor))
  (Utilities|FlowControl|DoOnce false
    (:Completed
      (Default|UpdateScore _asplayer_character)
      (Utilities|Time|SetTimerbyEvent (delegate Custom|Destroy) 5.0 true))))

(event OnComponentBeginOverlap(deathbox)
  (params (OverlappedComponent :type Primitive%20Component%20Object%20Reference) (OtherActor :type Actor%20Object%20Reference) (OtherComp :type Primitive%20Component%20Object%20Reference) (OtherBodyIndex :type Integer) (bFromSweep :type Boolean) (SweepResult :type Hit%20Result%20Structure%20%28by%20ref%29))
  (bind _asplayer_character (Utilities|Casting|CastToPlayerCharacter OtherActor))
  (Default|DeathOffScreen _asplayer_character))

(event OnComponentBeginOverlap(deathbox1)
  (params (OverlappedComponent :type Primitive%20Component%20Object%20Reference) (OtherActor :type Actor%20Object%20Reference) (OtherComp :type Primitive%20Component%20Object%20Reference) (OtherBodyIndex :type Integer) (bFromSweep :type Boolean) (SweepResult :type Hit%20Result%20Structure%20%28by%20ref%29))
  (bind _asplayer_character (Utilities|Casting|CastToPlayerCharacter OtherActor))
  (Default|DeathOffScreen (stale OnComponentBeginOverlap(deathbox) _asplayer_character)))

(event Custom|Destroy
  (if (> (- (.x (Transformation|GetActorLocation (stale OnComponentHit(Cube) _asplayer_character))) (.x (Transformation|GetActorLocation))) 2e+03)
    (Actor|DestroyActor)))

(event EventBeginPlay
  (Variables|Default|SetStartLocation (Transformation|GetWorldLocation (Variables|Default|GetStart)))
  (Variables|Default|SetEndLocation (Transformation|GetWorldLocation (Variables|Default|GetStart1)))
  (for _index (range 0 (Math|Float|Truncate (/ (Math|Vector|Distance(Vector) (Variables|Default|GetStartLocation) (Variables|Default|GetEndLocation)) 85.0)))
    (if (> (Math|Random|RandomFloat) 0.8)
      (Game|SpawnActorfromClass "/Game/CrossyRoadGame/Blueprints/TreeObstacles.TreeObstacles_C" (Math|Transform|MakeTransform (Math|Vector|MakeVector (.x (Variables|Default|GetStartLocation)) (+ (* _index 9e+01) (.Y (Math|Vector|BreakVector (Variables|Default|GetStartLocation)))) (.z (Variables|Default|GetStartLocation))) "0, 0, 0" "1,1,1") "Undefined" 0 0)
      (elif (< (Math|Random|RandomFloat) 0.01)
        (Game|SpawnActorfromClass "/Game/CrossyRoadGame/Blueprints/Coin.Coin_C" (Math|Transform|MakeTransform (Math|Vector|MakeVector (.x (Variables|Default|GetStartLocation)) (+ (* _index 9e+01) (.Y (Math|Vector|BreakVector (Variables|Default|GetStartLocation)))) (.z (Variables|Default|GetStartLocation))) "0, 0, 0" "0.500000,0.500000,0.500000") "Undefined" 0 0)))))

(fn ConstructionScript)