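; Terrain spawner actor for a Crossy Road-style game that lays out an endless track of terrain strips.
; On BeginPlay it places a run of strips along X: a fixed grass start, then random grass, road, railroad or water, with a river sound on water.
; A trigger placed partway along spawns the next TerrianSpawner past the end when the player first overlaps it, chaining segments endlessly.
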(event Custom|OnActorBeginOverlap_Event_0
  (params (OverlappedActor :type Actor%20Object%20Reference) (OtherActor :type Actor%20Object%20Reference))
  (bind _staticmesh (Variables|Default|GetStaticMesh))
  (bind _returnvalue (Transformation|GetWorldLocation _staticmesh))
  (Utilities|Casting|CastToPlayerCharacter OtherActor)
  (Utilities|FlowControl|DoOnce false
    (:Completed
      (bind _output_get (Variables|Default|SetSpawn%20Location (Math|Vector|MakeVector (+ 3.1e+03 (.x _returnvalue)) (.y _returnvalue) (.z _returnvalue))))
      (Game|SpawnActorfromClass "TerrianSpawner_C" (Math|Transform|MakeTransform _output_get "0, 0, 0" "1,1,1") "Undefined" 0 0))))

(event EventBeginPlay
  (bind _staticmesh (Variables|Default|GetStaticMesh))
  (bind _returnvalue (Transformation|GetWorldLocation _staticmesh))
  (for _index (range 0 30)
    (Variables|Default|SetSpawn%20Location (Math|Vector|MakeVector (+ (* _index 1e+02) (.x _returnvalue)) (.y _returnvalue) (.z _returnvalue)))
    (if (Math|Integer|InRange(Integer) _index 0 1)
      (Variables|Default|SetTerraintype "NewEnumerator0")
      (switch Utilities|FlowControl|Switch|SwitchonTerraintype (stale _output_get) :!label _label
        (:NewEnumerator0
          (Game|SpawnActorfromClass "/Game/CrossyRoadGame/Blueprints/TerrainstripGrass.TerrainstripGrass_C" (Math|Transform|MakeTransform (Variables|Default|GetSpawn%20Location) "0, 0, 0" "1,1,1") "AlwaysSpawn" 0 0))
        (:NewEnumerator4
          (Game|SpawnActorfromClass "/Game/CrossyRoadGame/Blueprints/TerrainstripGrasStart.TerrainstripGrasStart_C" (Math|Transform|MakeTransform (Variables|Default|GetSpawn%20Location) "0, 0, 0" "1,1,1") "AlwaysSpawn" 0 0)))
      (elif (== _index 2)
        (bind _output_get (Variables|Default|SetTerraintype "NewEnumerator4"))
        (goto _label)
        (elif (Math|Integer|InRange(Integer) _index 3 9)
          (switch int (Math|Random|RandomIntegerinRange 0 5) :!label _label_2
            (:0
              (Game|SpawnActorfromClass "/Game/CrossyRoadGame/Blueprints/TerrainstripGrass.TerrainstripGrass_C" (Math|Transform|MakeTransform (Variables|Default|GetSpawn%20Location) "0, 0, 0" "1,1,1") "AlwaysSpawn" 0 0))
            (:1
              (Game|SpawnActorfromClass "/Game/CrossyRoadGame/Blueprints/TerrainstripGrass1.TerrainstripGrass1_C" (Math|Transform|MakeTransform (Variables|Default|GetSpawn%20Location) "0, 0, 0" "1,1,1") "AlwaysSpawn" 0 0))
            (:2
              (Game|SpawnActorfromClass "/Game/CrossyRoadGame/Blueprints/TerrainstripRoad.TerrainstripRoad_C" (Math|Transform|MakeTransform (Variables|Default|GetSpawn%20Location) "0, 0, 0" "1,1,1") "AlwaysSpawn" 0 0 :!label _label_3))
            (:3
              (goto _label_3))
            (:4
              (Game|SpawnActorfromClass "/Game/CrossyRoadGame/Blueprints/TerrainstripRailroad.TerrainstripRailroad_C" (Math|Transform|MakeTransform (Variables|Default|GetSpawn%20Location) "0, 0, 0" "1,1,1") "Undefined" 0 0))
            (:5
              (Game|SpawnActorfromClass "/Game/CrossyRoadGame/Blueprints/water.water_C" (Math|Transform|MakeTransform (Variables|Default|GetSpawn%20Location) "0, 0, 0" "1,1,1") "AlwaysSpawn" 0 0)
              (Audio|PlaySoundatLocation "/Game/Sounds/CrossyRoadRiverCue.CrossyRoadRiverCue" (Variables|Default|GetSpawn%20Location) "0, 0, 0" 0.2 1.0 0.0 0 0 0)))
          (elif (== _index 10)
            (Game|SpawnActorfromClass "/Game/CrossyRoadGame/Blueprints/TerrainstripGrass.TerrainstripGrass_C" (Math|Transform|MakeTransform (Variables|Default|GetSpawn%20Location) "0, 0, 0" "1,1,1") "AlwaysSpawn" 0 0)
            (bind _returnvalue_2 (Game|SpawnActorfromClass "/Game/CrossyRoadGame/Blueprints/Collisionformore.Collisionformore_C" (Math|Transform|MakeTransform (Variables|Default|GetSpawn%20Location) "0, 0, 0" "1,1,1") "Undefined" 0 0))
            (EventDispatchers|AssignOnActorBeginOverlap _returnvalue_2 (delegate Custom|OnActorBeginOverlap_Event_0))
            (elif (Math|Integer|InRange(Integer) _index 11 30)
              (goto _label_2))))))))

(fn ConstructionScript)