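; TerrainstripGrasStart is a grass terrain strip for a Crossy Road-style game, apparently the starting variant.
; When a ThirdPersonCharacter first hits its Cube, a DoOnce gate lets it call that character's UpdateScore a single time.
; A disconnected graph would randomly spawn TreeObstacles along Y between the Start and Start1 components, but it never runs, and BeginPlay and the construction script are empty.
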(event OnComponentHit(Cube)
  (params (HitComponent :type Primitive%20Component%20Object%20Reference) (OtherActor :type Actor%20Object%20Reference) (OtherComp :type Primitive%20Component%20Object%20Reference) (NormalImpulse :type Vector :default "0, 0, 0") (Hit :type Hit%20Result%20Structure%20%28by%20ref%29))
  (bind _asthird_person_character (Utilities|Casting|CastToThirdPersonCharacter OtherActor))
  (Utilities|FlowControl|DoOnce false
    (:Completed
      (Default|UpdateScore _asthird_person_character))))

(event EventBeginPlay)

(fn ConstructionScript)