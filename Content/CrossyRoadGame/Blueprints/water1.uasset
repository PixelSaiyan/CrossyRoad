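; Water row actor for a Crossy Road-style game that scatters objects across itself, scores the player's crossing and cleans itself up.
; On BeginPlay it steps along Y over the span between two marker components, randomly spawning actors with random yaw in some slots.
; The first player overlap with Box updates the score and starts a looping timer that destroys the row once the player is far ahead in X.
; Two death boxes trigger the player's off-screen death.
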(event OnComponentBeginOverlap(deathbox)
  (params (OverlappedComponent :type Primitive%20Component%20Object%20Reference) (OtherActor :type Actor%20Object%20Reference) (OtherComp :type Primitive%20Component%20Object%20Reference) (OtherBodyIndex :type Integer) (bFromSweep :type Boolean) (SweepResult :type Hit%20Result%20Structure%20%28by%20ref%29))
  (bind _asplayer_character (Utilities|Casting|CastToPlayerCharacter (stale OnComponentBeginOverlap(deathbox1) OtherActor)))
  (Default|DeathOffScreen _asplayer_character))

(event OnComponentBeginOverlap(Box)
  (params (OverlappedComponent :type Primitive%20Component%20Object%20Reference) (OtherActor :type Actor%20Object%20Reference) (OtherComp :type Primitive%20Component%20Object%20Reference) (OtherBodyIndex :type Integer) (bFromSweep :type Boolean) (SweepResult :type Hit%20Result%20Structure%20%28by%20ref%29))
  (bind _asplayer_character (Utilities|Casting|CastToPlayerCharacter OtherActor))
  (Utilities|FlowControl|DoOnce false
    (:Completed
      (Default|UpdateScore _asplayer_character)
      (Utilities|Time|SetTimerbyEvent (delegate Custom|Destroy) 5.0 true))))

(event OnComponentBeginOverlap(Box1)
  (params (OverlappedComponent :type Primitive%20Component%20Object%20Reference) (OtherActor :type Actor%20Object%20Reference) (OtherComp :type Primitive%20Component%20Object%20Reference) (OtherBodyIndex :type Integer) (bFromSweep :type Boolean) (SweepResult :type Hit%20Result%20Structure%20%28by%20ref%29)))

(event OnComponentBeginOverlap(deathbox1)
  (params (OverlappedComponent :type Primitive%20Component%20Object%20Reference) (OtherActor :type Actor%20Object%20Reference) (OtherComp :type Primitive%20Component%20Object%20Reference) (OtherBodyIndex :type Integer) (bFromSweep :type Boolean) (SweepResult :type Hit%20Result%20Structure%20%28by%20ref%29))
  (bind _asplayer_character (Utilities|Casting|CastToPlayerCharacter OtherActor))
  (Default|DeathOffScreen _asplayer_character))

(event Custom|Destroy
  (if (> (- (.x (Transformation|GetActorLocation (stale OnComponentBeginOverlap(Box) _asplayer_character))) (.x (Transformation|GetActorLocation))) 2e+03)
    (Actor|DestroyActor)))

(event EventBeginPlay
  (Variables|Default|SetStart%20Location (Transformation|GetWorldLocation (Variables|Default|GetStart)))
  (Variables|Default|SetEnd%20Location (Transformation|GetWorldLocation (Variables|Default|GetStart1)))
  (for _index (range 0 (Math|Float|Truncate (/ (Math|Vector|Distance(Vector) (Variables|Default|GetStart%20Location) (Variables|Default|GetEnd%20Location)) 85.0)))
    (if (> (Math|Random|RandomFloat) 0.8)
      (Game|SpawnActorfromClass "/Game/CrossyRoadGame/Blueprints/Lilipad.Lilipad_C" (Math|Transform|MakeTransform (Math|Vector|MakeVector (.x (Variables|Default|GetStart%20Location)) (+ (* _index 9e+01) (.Y (Math|Vector|BreakVector (Variables|Default|GetStart%20Location)))) (.z (Variables|Default|GetStart%20Location))) (Math|Rotator|MakeRotator 0.0 0.0 (Math|Random|RandomFloatinRange 0.0 3.6e+02)) "1.500000,2.000000,1.000000") "Undefined" 0 0))))

(fn ConstructionScript)